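; BP_HorologiumMod_234 is a mod bootstrap actor that adds a debug camera to the game.
; On Tick it waits until the player pawn, controller and camera manager are valid, then spawns BP_DebugCamera, sets its movement and interpolation speeds, and destroys itself.
; The camera spawns without a meaningful transform, as it takes on the current POV when first enabled.
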(event `self.ReceiveTick`
  (params (DeltaSeconds :type "Float (single-precision)"))
  (bind _returnvalue (`GameplayStatics.GetPlayerController` 0))
  (if (and (`KismetSystemLibrary.IsValid` (`GameplayStatics.GetPlayerPawn` 0)) (`KismetSystemLibrary.IsValid` _returnvalue) (`KismetSystemLibrary.IsValid` (`PlayerController.PlayerCameraManager` _returnvalue)))
    ;[1 1 1] Location and Rotation will be set to current POV when we enable it for the first time
    (bind _returnvalue_2 (`|SpawnActorFromClass` "/Game/DebugCamera/BP_DebugCamera.BP_DebugCamera_C" (`KismetMathLibrary.MakeTransform` (0.0 0.0 0.0)) "Undefined" "OverrideRootScale" null null))
    (set `/Game/DebugCamera/BP_DebugCamera.MovementMultiplier` 10.0 _returnvalue_2)
    (set `/Game/DebugCamera/BP_DebugCamera.InterpSpeed` 10.0 _returnvalue_2)
    (`self.K2_DestroyActor`)))

(fn `UserConstructionScript`)