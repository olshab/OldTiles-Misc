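; Mod actor for Horologium that puts the local player into Unreal's debug camera when T is pressed.
; It enables input on BeginPlay, then EnableDebugCamera spawns a DebugCameraController once, caches it and activates it from the original controller.
; SwitchController hands over control by directly rewiring the Player and PlayerController references.
; An alternative BP_DebugCamera spawn is left unwired, and the Tick key-release check does nothing.
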(event `self.ReceiveBeginPlay`
  (`self.EnableInput` (`GameplayStatics.GetPlayerController` 0)))

(event `self.ReceiveTick`
  (params (DeltaSeconds :type "Float (single-precision)"))
  (if (`PlayerController.WasInputKeyJustReleased` (`GameplayStatics.GetPlayerController` 0) "T")
    _))

(event `Key|T`
  (params (Key :type "Key Structure"))
  (bind _returnvalue (`GameplayStatics.GetPlayerController` 0))
  (:`Pressed`
    (if (and (`KismetSystemLibrary.IsValid` (`GameplayStatics.GetPlayerPawn` 0)) (`KismetSystemLibrary.IsValid` _returnvalue) (`KismetSystemLibrary.IsValid` (`PlayerController.PlayerCameraManager` _returnvalue)))
      (`KismetSystemLibrary.PrintString` (`KismetSystemLibrary.GetDisplayName` (`PlayerController.Player` (`GameplayStatics.GetPlayerController` 0))))
      (`self.EnableDebugCamera`))))

(fn `EnableDebugCamera`
  (bind _returnvalue (`GameplayStatics.GetPlayerController` 0))
  (bind _debugcameracontrollerref (`self.DebugCameraControllerRef`))
  (if (and (`KismetSystemLibrary.IsValid` _returnvalue) (`KismetSystemLibrary.IsValid` (`PlayerController.Player` _returnvalue)) (`Controller.IsLocalPlayerController` _returnvalue))
    (`/Engine/EditorBlueprintResources/StandardMacros.IsValid` (`self.DebugCameraControllerRef`)
      (:`Is Valid`
        _)
      (:`Is Not Valid`
        (bind _returnvalue_2 (`|SpawnActorFromClass` "/Game/DebugCamera/DebugCameraController.DebugCameraController_C" (`KismetMathLibrary.MakeTransform` (0.0 0.0 0.0)) "Undefined" "OverrideRootScale" null (`self.GetInstigator` (`GameplayStatics.GetPlayerController` 0))))
        (set `self.DebugCameraControllerRef` _returnvalue_2)))
    (`/Engine/EditorBlueprintResources/StandardMacros.IsValid` _debugcameracontrollerref
      (:`Is Valid`
        (`/Game/DebugCamera/DebugCameraController.OnActivate` _debugcameracontrollerref (`GameplayStatics.GetPlayerController` 0))
        (`self.SwitchController` (`PlayerController.Player` (`GameplayStatics.GetPlayerController` 0)) (`self.DebugCameraControllerRef`))))))

(fn `SwitchController`
  (params (Player :type "Player Object Reference") (PC :type "PlayerController Object Reference"))
  (bind _playercontroller (`Player.PlayerController` Player))
  (`/Engine/EditorBlueprintResources/StandardMacros.IsValid` _playercontroller
    (:`Is Valid`
      (set `PlayerController.Player` null _playercontroller)
      (set `PlayerController.Player` Player PC)
      (set `Player.PlayerController` PC Player))))

(fn `UserConstructionScript`)